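; BP_Lift is a lift prop that moves a mini elevator platform up or down when something overlaps its Interaction component.
; The UpDownAnimation timeline drives the platform's relative Z, playing forward from the bottom and in reverse from the end when at the top.
; A Moving flag ignores overlaps during travel, and OnBottom flips when the timeline finishes to set the next direction.
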(event OnComponentBeginOverlap(Interaction)
  (params (OverlappedComponent :type Primitive%20Component%20Object%20Reference) (OtherActor :type Actor%20Object%20Reference) (OtherComp :type Primitive%20Component%20Object%20Reference) (OtherBodyIndex :type Integer) (bFromSweep :type Boolean) (SweepResult :type Hit%20Result%20Structure%20%28by%20ref%29))
  (bind _minielevator_platform (Variables|Default|GetMiniElevator_Platform))
  (bind _relativelocation (Variables|/Script/Engine.SceneComponent|GetRelativeLocation _minielevator_platform))
  (if (not (Variables|Default|GetMoving))
    (if (Variables|Default|GetOnBottom)
      (Variables|Default|SetMoving true)
      (bind _newtrack_0 (Timeline|UpDownAnimation Play)
        (:Update
          (Transformation|SetRelativeLocation _minielevator_platform (Math|Vector|MakeVector (.x _relativelocation) (.y _relativelocation) _newtrack_0) false false))
        (:Finished
          (if (Variables|Default|GetOnBottom)
            (Variables|Default|SetOnBottom false)
            (else
              (Variables|Default|SetOnBottom true)))
          (Variables|Default|SetMoving false)))
      (else
        (Variables|Default|SetMoving true)
        (Timeline|UpDownAnimation ReverseFromEnd)))))

(event EventBeginPlay)

(fn ConstructionScript)