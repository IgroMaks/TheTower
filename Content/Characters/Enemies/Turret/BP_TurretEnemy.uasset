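; Enemy turret that locks onto the player while they are inside its detection sphere.
; While locked, Tick yaws the skeletal mesh toward the player and aims two beam particles at them; per-gun update events are empty.
; Overlap begin and end toggle beam visibility and start or clear two looping, staggered timers.
; Each timer spawns a BP_Bullet_Enemy volley from four arrow components on the right or left side.
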(event OnComponentBeginOverlap(Sphere)
  (params (OverlappedComponent :type Primitive%20Component%20Object%20Reference) (OtherActor :type Actor%20Object%20Reference) (OtherComp :type Primitive%20Component%20Object%20Reference) (OtherBodyIndex :type Integer) (bFromSweep :type Boolean) (SweepResult :type Hit%20Result%20Structure%20%28by%20ref%29))
  (if (== OtherActor (Game|GetPlayerCharacter 0))
    (Variables|Default|SetTargetLocked true)
    (CallFunction|ReFire)
    (Rendering|ToggleVisibility (Variables|Default|GetPS_TurretBeam1) false)))

(event OnComponentEndOverlap(Sphere)
  (params (OverlappedComponent :type Primitive%20Component%20Object%20Reference) (OtherActor :type Actor%20Object%20Reference) (OtherComp :type Primitive%20Component%20Object%20Reference) (OtherBodyIndex :type Integer))
  (if (== OtherActor (Game|GetPlayerCharacter 0))
    (Variables|Default|SetTargetLocked false)
    (CallFunction|OutFire)
    (Rendering|ToggleVisibility (Variables|Default|GetPS_TurretBeam1) false)))

(event Custom|UpdateGunsLeft)

(event Custom|UpdateGunRight)

(event Custom|Left
  (bind _arrow4 (Variables|Default|GetArrow4))
  (bind _arrow6 (Variables|Default|GetArrow6))
  (bind _arrow7 (Variables|Default|GetArrow7))
  (bind _arrow5 (Variables|Default|GetArrow5))
  (bind _returnvalue (Transformation|GetWorldTransform _arrow4))
  (bind _returnvalue_2 (Transformation|GetWorldTransform _arrow6))
  (bind _returnvalue_3 (Transformation|GetWorldTransform _arrow7))
  (bind _returnvalue_4 (Transformation|GetWorldTransform _arrow5))
  (Utilities|FlowControl|Sequence
    (:then_0
      ;[1 1 1] Left
      (Game|SpawnActorfromClass "/Game/Blueprints/Weapon/BlueprintsBullet/BP_Bullet_Enemy.BP_Bullet_Enemy_C" (Math|Transform|MakeTransform (.location _returnvalue) (.rotation _returnvalue) "1,1,1") "Undefined" 0 0))
    (:then_1
      (Game|SpawnActorfromClass "/Game/Blueprints/Weapon/BlueprintsBullet/BP_Bullet_Enemy.BP_Bullet_Enemy_C" (Math|Transform|MakeTransform (.location _returnvalue_2) (.rotation _returnvalue_2) "1,1,1") "Undefined" 0 0))
    (:then_2
      (Game|SpawnActorfromClass "/Game/Blueprints/Weapon/BlueprintsBullet/BP_Bullet_Enemy.BP_Bullet_Enemy_C" (Math|Transform|MakeTransform (.location _returnvalue_3) (.rotation _returnvalue_3) "1,1,1") "Undefined" 0 0))
    (:then_3
      (Game|SpawnActorfromClass "/Game/Blueprints/Weapon/BlueprintsBullet/BP_Bullet_Enemy.BP_Bullet_Enemy_C" (Math|Transform|MakeTransform (.location _returnvalue_4) (.rotation _returnvalue_4) "1,1,1") "Undefined" 0 0))))

(event Custom|UpdateRotation
  (bind _turretprototypeskeletal (Variables|Default|GetTurretPrototypeSkeletal))
  (Transformation|SetWorldRotation _turretprototypeskeletal (Math|Rotator|MakeRotator 0.0 0.0 (+ (.yaw (Math|Rotator|FindLookatRotation (Transformation|GetActorLocation (Components|GetOwner _turretprototypeskeletal)) (Transformation|GetActorLocation (Game|GetPlayerCharacter 0)))) -9e+01)) false false))

(event Custom|Right
  (bind _arrow (Variables|Default|GetArrow))
  (bind _arrow1 (Variables|Default|GetArrow1))
  (bind _arrow2 (Variables|Default|GetArrow2))
  (bind _arrow3 (Variables|Default|GetArrow3))
  (bind _returnvalue (Transformation|GetWorldTransform _arrow))
  (bind _returnvalue_2 (Transformation|GetWorldTransform _arrow1))
  (bind _returnvalue_3 (Transformation|GetWorldTransform _arrow2))
  (bind _returnvalue_4 (Transformation|GetWorldTransform _arrow3))
  (Utilities|FlowControl|Sequence
    (:then_0
      ;[1 1 1] Right
      (Game|SpawnActorfromClass "/Game/Blueprints/Weapon/BlueprintsBullet/BP_Bullet_Enemy.BP_Bullet_Enemy_C" (Math|Transform|MakeTransform (.location _returnvalue) (.rotation _returnvalue) "1,1,1") "Undefined" 0 0))
    (:then_1
      (Game|SpawnActorfromClass "/Game/Blueprints/Weapon/BlueprintsBullet/BP_Bullet_Enemy.BP_Bullet_Enemy_C" (Math|Transform|MakeTransform (.location _returnvalue_2) (.rotation _returnvalue_2) "1,1,1") "Undefined" 0 0))
    (:then_2
      (Game|SpawnActorfromClass "/Game/Blueprints/Weapon/BlueprintsBullet/BP_Bullet_Enemy.BP_Bullet_Enemy_C" (Math|Transform|MakeTransform (.location _returnvalue_3) (.rotation _returnvalue_3) "1,1,1") "Undefined" 0 0))
    (:then_3
      (Game|SpawnActorfromClass "/Game/Blueprints/Weapon/BlueprintsBullet/BP_Bullet_Enemy.BP_Bullet_Enemy_C" (Math|Transform|MakeTransform (.location _returnvalue_4) (.rotation _returnvalue_4) "1,1,1") "Undefined" 0 0))))

(event Custom|ReFire
  (bind _returnvalue (Utilities|Time|SetTimerbyEvent (delegate Custom|Right) 0.5 true))
  (Utilities|FlowControl|Delay 0.2)
  (bind _returnvalue_2 (Utilities|Time|SetTimerbyEvent (delegate Custom|Left) 0.5 true)))

(event Custom|OutFire
  (Utilities|Time|ClearandInvalidateTimerbyHandle (stale Custom|ReFire _returnvalue))
  (Utilities|Time|ClearandInvalidateTimerbyHandle (stale Custom|ReFire _returnvalue_2)))

(event EventTick
  (params (DeltaSeconds :type Float%20%28single-precision%29))
  (bind _returnvalue (Game|GetPlayerCharacter 0))
  (bind _returnvalue_2 (Transformation|GetActorLocation _returnvalue))
  (if (Variables|Default|GetTargetLocked)
    (CallFunction|UpdateRotation)
    (Utilities|FlowControl|Sequence
      (:then_0
        (CallFunction|UpdateGunRight)
        (Class|ParticleSystemComponent|SetBeamTargetPoint (Variables|Default|GetPS_TurretBeam1) 0 _returnvalue_2))
      (:then_1
        (CallFunction|UpdateGunsLeft)
        (Class|ParticleSystemComponent|SetBeamTargetPoint (Variables|Default|GetParticleSystem) 0 _returnvalue_2)))))

(fn ConstructionScript)