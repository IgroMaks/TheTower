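; Enemy character that chases the hero, shoots bullets and dies from hero bullet hits.
; PawnSensing sends it to the player hero with AI MoveTo whenever it sees a pawn.
; Custom events start and clear a looping timer that spawns enemy bullets with sound at the arrow; nothing here calls them.
; Capsule overlaps with hero bullets reduce health, update a widget health bar and, at zero, spawn a death effect and destroy it.
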(event OnComponentBeginOverlap(CapsuleComponent)
  (params (OverlappedComponent :type Primitive%20Component%20Object%20Reference) (OtherActor :type Actor%20Object%20Reference) (OtherComp :type Primitive%20Component%20Object%20Reference) (OtherBodyIndex :type Integer) (bFromSweep :type Boolean) (SweepResult :type Hit%20Result%20Structure%20%28by%20ref%29))
  (bind _asbp_bullet_hero (Utilities|Casting|CastToBP_Bullet_Hero OtherActor))
  (CallFunction|GetDamage (Variables|/Game/Blueprints/Weapon/BlueprintsBullet/BP_Bullet_Master.BP_Bullet_Master_C|GetDamage _asbp_bullet_hero))
  (Default|ImpactSpawn _asbp_bullet_hero)
  (Actor|DestroyActor _asbp_bullet_hero)
  (Progress|SetPercent (Variables|/Game/Widgets/WBP_UIEnemy.WBP_UIEnemy_C|GetProgressBar_23 (stale EventBeginPlay _returnvalue)) (/ (Variables|Default|GetHealth) (Variables|Default|GetMaxHealth))))

(event OnSeePawn(PawnSensing)
  (params (Pawn :type Pawn%20Object%20Reference))
  (bind _asbp_hero_character (Utilities|Casting|CastToBp_HeroCharacter (Game|GetPlayerCharacter 0)))
  (AI|AIMoveTo self "0, 0, 0" _asbp_hero_character 5.0 false))

(event Custom|FireDamage)

(event Custom|FireToHero
  (Game|SpawnActorfromClass "/Game/Blueprints/Weapon/BlueprintsBullet/BP_BulletEnemy.BP_BulletEnemy_C" (Transformation|GetWorldTransform (Variables|Default|GetArrow1)) "Undefined" 0 0)
  (Audio|PlaySoundatLocation "/Game/SFX/Weapon/Pistol/WPN_PistolFire.WPN_PistolFire" "0, 0, 0" "0, 0, 0" 0.1 1.0 0.0 0 0 0))

(event Custom|ReFireToEnemy
  (bind _returnvalue (Utilities|Time|SetTimerbyEvent (delegate Custom|FireToHero) (/ 1.0 5.0) true)))

(event Custom|OutFire
  (Utilities|Time|ClearandInvalidateTimerbyHandle (stale Custom|ReFireToEnemy _returnvalue)))

(event EventBeginPlay
  (Utilities|FlowControl|Sequence
    (:then_0
      (Variables|Default|SetHealth (Variables|Default|GetMaxHealth)))
    (:then_1
      (bind _returnvalue (UserInterface|CreateWidget "/Game/Widgets/WBP_UIEnemy.WBP_UIEnemy_C"))
      (UserInterface|SetWidget (Variables|Default|GetWidget) _returnvalue))))

(fn ConstructionScript)

(fn GetDamage
  (params (Damage :type Float%20%28single-precision%29))
  (bind _output_get (Variables|Default|SetHealth (- (Variables|Default|GetHealth) Damage)))
  (if (<= _output_get 0.0)
    (Effects|SpawnEmitteratLocation "/Game/VFX/PS_EmenyDeath.PS_EmenyDeath" (Transformation|GetWorldLocation (Variables|Default|GetArrow1)))
    (Actor|DestroyActor)))