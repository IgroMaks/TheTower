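; Hero weapon actor holding blade, pistol, shotgun, rifle and laser, with ChangeWeapon toggling mesh visibility.
; Pistol and rifle fire on looping timers at game-instance fire rates, while the shotgun sprays six randomly spread bullets behind a delayed DoOnce.
; The laser timer drains ammo and line-traces, spawning impacts on static meshes without applying damage.
; Ammo lives in the game instance, but the pistol's check compares zero to zero, so it never fires.
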(event Custom|ReFireLaser
  (bind _arrow2 (Variables|Default|GetArrow2))
  (bind _returnvalue (Transformation|GetWorldTransform _arrow2))
  (bind _returnvalue_2 (Effects|SpawnEmitteratLocation "/Game/VFX/PS_Laser.PS_Laser" (.location _returnvalue) (.rotation _returnvalue)))
  (bind _returnvalue_3 (Utilities|Time|SetTimerbyEvent (delegate Custom|FireLaser1) 0.25 true)))

(event Custom|FireRifle
  (bind _instanceref (Variables|Default|GetInstanceRef))
  (bind _assultriflemuzzle (Variables|Default|GetAssultRifleMuzzle))
  (bind _returnvalue (Transformation|GetWorldTransform _assultriflemuzzle))
  (bind _returnvalue_2 (Transformation|GetWorldTransform _assultriflemuzzle))
  ;[1 1 1] Rifle
  (if (> (Variables|/Game/Blueprints/ThirdPersonBP/Blueprints/MainGameInstance.MainGameInstance_C|GetAmmoRifle (Variables|Default|GetInstanceRef)) 0)
    (Game|SpawnActorfromClass "/Game/Blueprints/Weapon/BlueprintsBullet/BP_Bullet_Hero.BP_Bullet_Hero_C" (Math|Transform|MakeTransform (.location _returnvalue) (.rotation _returnvalue) "1,1,1") "AlwaysSpawn" 0 0)
    (bind _returnvalue_3 (Game|SpawnActorfromClass "/Game/VFX/BlueprintsVFX/BP_ShootVFX_Hero.BP_ShootVFX_Hero_C" (Math|Transform|MakeTransform (.location _returnvalue_2) (.rotation _returnvalue_2) "1,1,1") "AlwaysSpawn" 0 0))
    (Transformation|AttachComponentToComponent _returnvalue_3 _assultriflemuzzle "None" "SnapToTarget" "SnapToTarget" "SnapToTarget" true)
    (bind _result (Math|Integer|DecrementInt (Variables|/Game/Blueprints/ThirdPersonBP/Blueprints/MainGameInstance.MainGameInstance_C|GetAmmoRifle _instanceref))
      (:%20%20
        (Variables|/Game/Blueprints/ThirdPersonBP/Blueprints/MainGameInstance.MainGameInstance_C|SetAmmoRifle _instanceref _result)
        (Audio|PlaySoundatLocation "/Game/SFX/Weapon/AssaultRifle/WPN_Rifle.WPN_Rifle" "0, 0, 0" "0, 0, 0" 0.1 1.0 0.0 0 0 0)))
    (else
      (Utilities|Time|ClearandInvalidateTimerbyHandle (stale Custom|ReFireRifle _returnvalue)))))

(event Custom|Fire%20Shotgun
  (bind _arrow1 (Variables|Default|GetArrow1))
  (bind _instanceref (Variables|Default|GetInstanceRef))
  (bind _arrow1_2 (Variables|Default|GetArrow1))
  (bind _min (Variables|Default|GetMin))
  (bind _max (Variables|Default|GetMax))
  (bind _returnvalue (Transformation|GetWorldLocation _arrow1))
  (bind _returnvalue_2 (Transformation|GetWorldRotation _arrow1))
  ;[1 1 1] Shotgun
  (Variables|Default|SetFireSpeed (Utilities|Array|Get(acopy) (Variables|/Game/Blueprints/ThirdPersonBP/Blueprints/MainGameInstance.MainGameInstance_C|GetAll_SpeedFireWeapon (Variables|Default|GetInstanceRef)) 1))
  (Utilities|FlowControl|DoOnce false :!label _label
    (:Completed
      (if (>= (Variables|/Game/Blueprints/ThirdPersonBP/Blueprints/MainGameInstance.MainGameInstance_C|GetAmmoShotgun _instanceref) 6)
        (Utilities|FlowControl|Sequence
          (:then_0
            (Game|SpawnActorfromClass "/Game/Blueprints/Weapon/BlueprintsBullet/BP_Bullet_Hero.BP_Bullet_Hero_C" (Math|Transform|MakeTransform _returnvalue (Math|Rotator|MakeRotator (.roll _returnvalue_2) (+ (.pitch _returnvalue_2) (Math|Random|RandomFloatinRange _min _max)) (+ (.yaw _returnvalue_2) (Math|Random|RandomFloatinRange _min _max))) "1,1,1") "Undefined" 0 0)
            (Game|SpawnActorfromClass "/Game/Blueprints/Weapon/BlueprintsBullet/BP_Bullet_Hero.BP_Bullet_Hero_C" (Math|Transform|MakeTransform _returnvalue (Math|Rotator|MakeRotator (.roll _returnvalue_2) (+ (.pitch _returnvalue_2) (Math|Random|RandomFloatinRange _min _max)) (+ (.yaw _returnvalue_2) (Math|Random|RandomFloatinRange _min _max))) "1,1,1") "Undefined" 0 0)
            (Game|SpawnActorfromClass "/Game/Blueprints/Weapon/BlueprintsBullet/BP_Bullet_Hero.BP_Bullet_Hero_C" (Math|Transform|MakeTransform _returnvalue (Math|Rotator|MakeRotator (.roll _returnvalue_2) (+ (.pitch _returnvalue_2) (Math|Random|RandomFloatinRange _min _max)) (+ (.yaw _returnvalue_2) (Math|Random|RandomFloatinRange _min _max))) "1,1,1") "Undefined" 0 0)
            (Variables|/Game/Blueprints/ThirdPersonBP/Blueprints/MainGameInstance.MainGameInstance_C|SetAmmoShotgun _instanceref (- (Variables|/Game/Blueprints/ThirdPersonBP/Blueprints/MainGameInstance.MainGameInstance_C|GetAmmoShotgun _instanceref) 6))
            (Utilities|FlowControl|Delay (/ 1.0 (Variables|Default|GetFireSpeed)))
            (goto _label Reset))
          (:then_1
            (Game|SpawnActorfromClass "/Game/Blueprints/Weapon/BlueprintsBullet/BP_Bullet_Hero.BP_Bullet_Hero_C" (Math|Transform|MakeTransform _returnvalue (Math|Rotator|MakeRotator (.roll _returnvalue_2) (+ (.pitch _returnvalue_2) (Math|Random|RandomFloatinRange _min _max)) (+ (.yaw _returnvalue_2) (Math|Random|RandomFloatinRange _min _max))) "1,1,1") "Undefined" 0 0)
            (Game|SpawnActorfromClass "/Game/Blueprints/Weapon/BlueprintsBullet/BP_Bullet_Hero.BP_Bullet_Hero_C" (Math|Transform|MakeTransform _returnvalue (Math|Rotator|MakeRotator (.roll _returnvalue_2) (+ (.pitch _returnvalue_2) (Math|Random|RandomFloatinRange _min _max)) (+ (.yaw _returnvalue_2) (Math|Random|RandomFloatinRange _min _max))) "1,1,1") "Undefined" 0 0)
            (Game|SpawnActorfromClass "/Game/Blueprints/Weapon/BlueprintsBullet/BP_Bullet_Hero.BP_Bullet_Hero_C" (Math|Transform|MakeTransform _returnvalue (Math|Rotator|MakeRotator (.roll _returnvalue_2) (+ (.pitch _returnvalue_2) (Math|Random|RandomFloatinRange _min _max)) (+ (.yaw _returnvalue_2) (Math|Random|RandomFloatinRange _min _max))) "1,1,1") "Undefined" 0 0)
            (bind _returnvalue_3 (Game|SpawnActorfromClass "/Game/VFX/BlueprintsVFX/BP_ShootVFX_Hero.BP_ShootVFX_Hero_C" (Transformation|GetWorldTransform _arrow1_2) "Undefined" 0 0))
            (Transformation|AttachComponentToComponent _returnvalue_3 _arrow1_2 "None" "SnapToTarget" "SnapToTarget" "SnapToTarget" true)
            (Audio|PlaySoundatLocation "/Game/SFX/Weapon/Shotgun/ShotGunTest.ShotGunTest" "0, 0, 0" "0, 0, 0" 0.1 1.0 0.0 0 0 0)))))))

(event Custom|FirePistol
  (bind _arrow (Variables|Default|GetArrow))
  ;[1 1 1] Pistol
  (if (> 0 0)
    (Game|SpawnActorfromClass "/Game/Blueprints/Weapon/BlueprintsBullet/BP_Bullet_Hero.BP_Bullet_Hero_C" (Transformation|GetWorldTransform (Variables|Default|GetArrow)) "Undefined" 0 0)
    (bind _returnvalue (Game|SpawnActorfromClass "/Game/VFX/BlueprintsVFX/BP_ShootVFX_Hero.BP_ShootVFX_Hero_C" (Transformation|GetWorldTransform _arrow) "AlwaysSpawn" 0 0))
    (Transformation|AttachComponentToComponent _returnvalue _arrow "None" "SnapToTarget" "SnapToTarget" "SnapToTarget" true)
    (Math|Integer|DecrementInt 0
      (:%20%20
        (Variables|/Game/Blueprints/ThirdPersonBP/Blueprints/MainGameInstance.MainGameInstance_C|SetAmmo_All (Variables|Default|GetInstanceRef) 0)
        (Audio|PlaySoundatLocation "/Game/SFX/Weapon/Pistol/WPN_PistolFire.WPN_PistolFire" "0, 0, 0" "0, 0, 0" 0.1 1.0 0.0 0 0 0)))
    (else
      (Utilities|Time|ClearandInvalidateTimerbyHandle (stale Custom|ReFirePistol _returnvalue)))))

(event Custom|OutFireLaser
  (Components|DestroyComponent (stale Custom|ReFireLaser _returnvalue_2))
  (Utilities|Time|ClearandInvalidateTimerbyHandle (stale Custom|ReFireLaser _returnvalue_3)))

(event Custom|ReFireRifle
  ;[1 1 1] Rifle
  (bind _output_get (Variables|Default|SetFireSpeed (Utilities|Array|Get(acopy) (Variables|/Game/Blueprints/ThirdPersonBP/Blueprints/MainGameInstance.MainGameInstance_C|GetAll_SpeedFireWeapon (Variables|Default|GetInstanceRef)) 2)))
  (CallFunction|FireRifle)
  (Utilities|FlowControl|DoOnce false :!label _label
    (:Completed
      (bind _returnvalue (Utilities|Time|SetTimerbyEvent (delegate Custom|FireRifle) (/ 1.0 _output_get) true))
      (Utilities|FlowControl|Delay (/ 1.0 _output_get))
      (goto _label Reset))))

(event Custom|OutFireRifle
  ;[1 1 1] Rifle
  (Utilities|Time|ClearandInvalidateTimerbyHandle (stale Custom|ReFireRifle _returnvalue)))

(event Custom|ReFirePistol
  ;[1 1 1] Pistol
  (Variables|Default|SetFireSpeed (Utilities|Array|Get(acopy) (Variables|/Game/Blueprints/ThirdPersonBP/Blueprints/MainGameInstance.MainGameInstance_C|GetAll_SpeedFireWeapon (Variables|Default|GetInstanceRef))))
  (Utilities|FlowControl|DoOnce false :!label _label
    (:Completed
      (CallFunction|FirePistol)
      (bind _returnvalue (Utilities|Time|SetTimerbyEvent (delegate Custom|FirePistol) (/ 1.0 (Variables|Default|GetFireSpeed)) true))
      (Utilities|FlowControl|Delay (/ 1.0 (Variables|Default|GetFireSpeed)))
      (goto _label Reset))))

(event Custom|OutFirePistol
  ;[1 1 1] Pistol
  (Utilities|Time|ClearandInvalidateTimerbyHandle (stale Custom|ReFirePistol _returnvalue)))

(event Custom|FireLaser1
  (bind _arrow2 (Variables|Default|GetArrow2))
  (bind _instanceref (Variables|Default|GetInstanceRef))
  (bind _returnvalue (Transformation|GetWorldLocation _arrow2))
  (Utilities|FlowControl|Sequence
    (:then_0
      (bind _result (Math|Integer|DecrementInt (Variables|/Game/Blueprints/ThirdPersonBP/Blueprints/MainGameInstance.MainGameInstance_C|GetAmmoLaser _instanceref))
        (:%20%20
          (bind _output_get (Variables|/Game/Blueprints/ThirdPersonBP/Blueprints/MainGameInstance.MainGameInstance_C|SetAmmoLaser _instanceref _result))
          (if (<= _output_get 0)
            (CallFunction|OutFireLaser)))))
    (:then_1
      (bind (_outhit _returnvalue_2) (Collision|LineTraceByChannel _returnvalue (+ _returnvalue (* (Math|Vector|GetForwardVector _arrow2) 5e+02)) "TraceTypeQuery1" false 0 "None"))
      (if _returnvalue_2
        (bind _asstatic_mesh_actor (Utilities|Casting|CastToStaticMeshActor (.HitActor (Collision|BreakHitResult _outhit))))
        (Effects|SpawnEmitteratLocation "/Game/VFX/PS_BulletImpact_Hero.PS_BulletImpact_Hero" (.Location (Collision|BreakHitResult _outhit)) (.rotation (Transformation|GetActorTransform _asstatic_mesh_actor)))))))

(event EventBeginPlay
  (bind _asbp_hero_character (Utilities|Casting|CastToBp_HeroCharacter (Game|GetPlayerCharacter 0)))
  (Variables|Default|SetHeroRef _asbp_hero_character)
  (bind _asmain_game_instance (Utilities|Casting|CastToMainGameInstance (Game|GetGameInstance)))
  (Variables|Default|SetInstanceRef _asmain_game_instance))

(fn ConstructionScript)

(fn ChangeWeapon
  (params (Weapon :type Integer))
  (switch int Weapon
    (:1
      (CallFunction|VisibleWeapon)
      (Rendering|ToggleVisibility (Variables|Default|GetBlade) false)
      (Variables|Default|SetEnumWeapon "NewEnumerator0"))
    (:2
      (CallFunction|VisibleWeapon)
      (Rendering|ToggleVisibility (Variables|Default|GetPistol) false)
      (Variables|Default|SetEnumWeapon "NewEnumerator1"))
    (:3
      (CallFunction|VisibleWeapon)
      (Rendering|ToggleVisibility (Variables|Default|GetShotGun) false)
      (Variables|Default|SetEnumWeapon "NewEnumerator6"))
    (:4
      (CallFunction|VisibleWeapon)
      (Rendering|ToggleVisibility (Variables|Default|GetWhite_AssaultRifle) false)
      (Variables|Default|SetEnumWeapon "NewEnumerator2"))
    (:6
      (CallFunction|VisibleWeapon)
      (Rendering|ToggleVisibility (Variables|Default|GetLaser) false)
      (Variables|Default|SetEnumWeapon "NewEnumerator3"))))

(fn VisibleWeapon
  (switch Utilities|FlowControl|Switch|SwitchonEnumWeapon (Variables|Default|GetEnumWeapon)
    (:NewEnumerator0
      (Rendering|ToggleVisibility (Variables|Default|GetBlade) false))
    (:NewEnumerator1
      (Rendering|ToggleVisibility (Variables|Default|GetPistol) false))
    (:NewEnumerator2
      (Rendering|ToggleVisibility (Variables|Default|GetWhite_AssaultRifle) false))
    (:NewEnumerator6
      (Rendering|ToggleVisibility (Variables|Default|GetShotGun) false))
    (:NewEnumerator3
      (Rendering|ToggleVisibility (Variables|Default|GetLaser) false))))