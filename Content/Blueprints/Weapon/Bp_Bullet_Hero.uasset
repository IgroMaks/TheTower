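; Hero bullet actor that damages Bp_EnemyCharacter on capsule overlap and destroys itself two seconds after spawning.
; A hit subtracts fixed Health, calls the enemy's FireDamage and toggles the particle system.
; After a longer delay it toggles particles back, destroys itself, then checks for death to spawn Bp_Drop and remove the enemy.
; The spawn lifetime expires before that delay completes, cutting off those later steps.
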(event OnComponentBeginOverlap(Capsule)
  (params (OverlappedComponent :type Primitive%20Component%20Object%20Reference) (OtherActor :type Actor%20Object%20Reference) (OtherComp :type Primitive%20Component%20Object%20Reference) (OtherBodyIndex :type Integer) (bFromSweep :type Boolean) (SweepResult :type Hit%20Result%20Structure%20%28by%20ref%29))
  (bind _asbp_enemy_character (Utilities|Casting|CastToBp_EnemyCharacter OtherActor))
  (if (== OtherActor _asbp_enemy_character)
    (Variables|/Game/Characters/Enemies/Enemy/Bp_EnemyCharacter.Bp_EnemyCharacter_C|SetHealth _asbp_enemy_character (- (Variables|/Game/Characters/Enemies/Enemy/Bp_EnemyCharacter.Bp_EnemyCharacter_C|GetHealth _asbp_enemy_character) 1e+01))
    (Default|FireDamage _asbp_enemy_character)
    (Components|Activation|ToggleActive (Variables|Default|GetParticleSystem))
    (Utilities|FlowControl|Delay 4.0)
    (Components|Activation|ToggleActive (Variables|Default|GetParticleSystem))
    (Actor|DestroyActor)
    (if (<= (Variables|/Game/Characters/Enemies/Enemy/Bp_EnemyCharacter.Bp_EnemyCharacter_C|GetHealth _asbp_enemy_character) 0.0)
      (Game|SpawnActorfromClass "/Game/Blueprints/Weapon/Bp_Drop.Bp_Drop_C" (Transformation|GetActorTransform _asbp_enemy_character) "AlwaysSpawn" 0 0)
      (Actor|DestroyActor _asbp_enemy_character))))

(event EventBeginPlay
  (Utilities|FlowControl|Delay 2.0)
  (Actor|DestroyActor))

(fn ConstructionScript)