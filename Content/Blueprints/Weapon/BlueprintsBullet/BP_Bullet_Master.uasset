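; BP_Bullet_Master is a bullet actor, named as the master for weapon bullets, with configurable material, light color and impact effect.
; The construction script applies the material to the bullet mesh and the color to its light.
; On hit, it spawns the ImpactParticle actor at the mesh location with yaw turned 180 degrees, ignoring collision, then destroys itself.
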(event Custom|ImpactSpawn
  (bind _bulletmesh (Variables|Default|GetBulletMesh))
  (bind _returnvalue (Transformation|GetWorldTransform _bulletmesh))
  (Game|SpawnActorfromClass (Variables|Default|GetImpactParticle) (Math|Transform|MakeTransform (.location _returnvalue) (Math|Rotator|MakeRotator (.roll (.rotation _returnvalue)) (.pitch (.rotation _returnvalue)) (+ (.yaw (.rotation _returnvalue)) 1.8e+02)) "1,1,1") "AlwaysSpawn" 0 0))

(event Collision|EventHit
  (params (MyComp :type Primitive%20Component%20Object%20Reference) (Other :type Actor%20Object%20Reference) (OtherComp :type Primitive%20Component%20Object%20Reference) (bSelfMoved :type Boolean) (HitLocation :type Vector :default "0, 0, 0") (HitNormal :type Vector :default "0, 0, 0") (NormalImpulse :type Vector :default "0, 0, 0") (Hit :type Hit%20Result%20Structure%20%28by%20ref%29))
  (CallFunction|ImpactSpawn)
  (Actor|DestroyActor))

(fn ConstructionScript
  (Rendering|Components|Light|SetLightColor (Variables|Default|GetBulletLight) (Variables|Default|GetLight%20Color) true)
  (Rendering|Material|SetMaterial (Variables|Default|GetBulletMesh) 0 (Variables|Default|GetBullet%20Material)))