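; BP_DinamoBullet_Hero is a hero projectile that grows its Sphere while charging, then toggles its ProjectileMovement.
; LoopBullet starts a looping timer whose Scale event enlarges the sphere in small steps.
; Reaching the target scale stops the timer and toggles movement.
; UnPress does the same without checking scale, so it can toggle movement again after a full charge.
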(event Custom|LoopBullet
  (bind _returnvalue (Utilities|Time|SetTimerbyEvent (delegate Custom|+Scale) 0.1 true)))

(event Custom|+Scale
  (bind _sphere (Variables|Default|GetSphere))
  (bind _relativescale3d (Variables|/Script/Engine.SceneComponent|GetRelativeScale3D _sphere))
  (Transformation|SetRelativeScale3D _sphere (+ _relativescale3d 0.01))
  (if (Math|Vector|Equal(Vector) _relativescale3d "5.000000,5.000000,5.000000" 0.0001)
    (Utilities|Time|ClearandInvalidateTimerbyHandle (stale Custom|LoopBullet _returnvalue))
    (Components|Activation|ToggleActive (Variables|Default|GetProjectileMovement))))

(event Custom|UnPress
  (Utilities|Time|ClearandInvalidateTimerbyHandle (stale Custom|LoopBullet _returnvalue))
  (Components|Activation|ToggleActive (Variables|Default|GetProjectileMovement)))

(fn ConstructionScript)