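; Enemy bullet projectile that damages the hero character on contact.
; It destroys itself after a one-second lifetime or when its capsule overlaps a Bp_HeroCharacter.
; On a hit it subtracts a fixed amount from the hero's Health and spawns BP_ParticleImpactEnemy at the hero's location.
; If that drops Health to zero or below, the bullet itself quits the game, with no separate death handling.
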(event OnComponentBeginOverlap(Capsule)
  (params (OverlappedComponent :type Primitive%20Component%20Object%20Reference) (OtherActor :type Actor%20Object%20Reference) (OtherComp :type Primitive%20Component%20Object%20Reference) (OtherBodyIndex :type Integer) (bFromSweep :type Boolean) (SweepResult :type Hit%20Result%20Structure%20%28by%20ref%29))
  (bind _asbp_hero_character (Utilities|Casting|CastToBp_HeroCharacter OtherActor))
  (Actor|DestroyActor)
  (bind _output_get (Variables|/Game/Blueprints/ThirdPersonBP/Blueprints/Bp_HeroCharacter.Bp_HeroCharacter_C|SetHealth _asbp_hero_character (- (Variables|/Game/Blueprints/ThirdPersonBP/Blueprints/Bp_HeroCharacter.Bp_HeroCharacter_C|GetHealth _asbp_hero_character) 0.5)))
  (Game|SpawnActorfromClass "/Game/VFX/BlueprintsVFX/BP_ParticleImpactEnemy.BP_ParticleImpactEnemy_C" (Math|Transform|MakeTransform (.location (Transformation|GetActorTransform _asbp_hero_character)) (Transformation|GetActorRotation) "1,1,1") "Undefined" 0 0)
  (if (<= _output_get 0.0)
    (Game|QuitGame 0 "Quit" false)))

(event EventBeginPlay
  (Utilities|FlowControl|Delay 1.0)
  (Actor|DestroyActor))

(fn ConstructionScript)