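; Melee blade weapon that deals repeated damage to an enemy character inside its hit box.
; Box overlap events cache the Bp_EnemyCharacter and toggle whether hits are enabled.
; ReHit, gated by a DoOnce, starts a looping timer that calls Hit about three times a second until OutHit clears it.
; Each enabled hit subtracts fixed health, calls FireDamage on the enemy and destroys it when health runs out.
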(event OnComponentBeginOverlap(Box)
  (params (OverlappedComponent :type Primitive%20Component%20Object%20Reference) (OtherActor :type Actor%20Object%20Reference) (OtherComp :type Primitive%20Component%20Object%20Reference) (OtherBodyIndex :type Integer) (bFromSweep :type Boolean) (SweepResult :type Hit%20Result%20Structure%20%28by%20ref%29))
  (bind _asbp_enemy_character (Utilities|Casting|CastToBp_EnemyCharacter OtherActor))
  (Variables|Default|SetEnableHit? true)
  (Development|PrintString "ENABLE"))

(event OnComponentEndOverlap(Box)
  (params (OverlappedComponent :type Primitive%20Component%20Object%20Reference) (OtherActor :type Actor%20Object%20Reference) (OtherComp :type Primitive%20Component%20Object%20Reference) (OtherBodyIndex :type Integer))
  (Utilities|Casting|CastToBp_EnemyCharacter OtherActor)
  (Variables|Default|SetEnableHit? false)
  (Development|PrintString "DISABLE"))

(event Custom|ReHit
  (bind _returnvalue (/ 1.0 3.0))
  (Utilities|FlowControl|DoOnce false :!label _label
    (:Completed
      (bind _returnvalue_2 (Utilities|Time|SetTimerbyEvent (delegate Custom|Hit) _returnvalue true))
      (Utilities|FlowControl|Delay _returnvalue)
      (CallFunction|Hit)
      (goto _label Reset))))

(event Custom|OutHit
  (bind _returnvalue (/ 1.0 3.0))
  (Utilities|Time|ClearandInvalidateTimerbyHandle (stale Custom|ReHit _returnvalue_2))
  (Utilities|FlowControl|DoOnce false) ; enters at Reset
)

(event Custom|Hit
  (if (Variables|Default|GetEnableHit?)
    (Variables|/Game/Characters/Enemies/Enemy/Bp_EnemyCharacter.Bp_EnemyCharacter_C|SetHealth (stale OnComponentBeginOverlap(Box) _asbp_enemy_character) (- (Variables|/Game/Characters/Enemies/Enemy/Bp_EnemyCharacter.Bp_EnemyCharacter_C|GetHealth (stale OnComponentBeginOverlap(Box) _asbp_enemy_character)) 1e+01))
    (Default|FireDamage (stale OnComponentBeginOverlap(Box) _asbp_enemy_character))
    (Development|PrintString "I Hit!")
    (if (<= (Variables|/Game/Characters/Enemies/Enemy/Bp_EnemyCharacter.Bp_EnemyCharacter_C|GetHealth (stale OnComponentBeginOverlap(Box) _asbp_enemy_character)) 0.0)
      (Actor|DestroyActor (stale OnComponentBeginOverlap(Box) _asbp_enemy_character)))))

(fn ConstructionScript)