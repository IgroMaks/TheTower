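; Pistol weapon Blueprint that spawns Bullet actors at its Arrow component's transform, with automatic repeat fire.
; ReFire fires immediately and starts a looping timer that calls Fire at a rate set by SpeedFire.
; A DoOnce, reset after one shot interval, gates ReFire against rapid retriggering.
; OutFire clears the timer to stop firing.
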(event Custom|Fire
  (Game|SpawnActorfromClass "/Game/Blueprints/Weapon/Bullet.Bullet_C" (Transformation|GetWorldTransform (Variables|Default|GetArrow)) "AlwaysSpawn" 0 0))

(event Custom|ReFire
  (bind _speedfire (Variables|Default|GetSpeedFire))
  (bind _returnvalue (/ 1.0 _speedfire))
  (Utilities|FlowControl|DoOnce false :!label _label
    (:Completed
      (bind _returnvalue_2 (Utilities|Time|SetTimerbyEvent (delegate Custom|Fire) _returnvalue true))
      (CallFunction|Fire)
      (Utilities|FlowControl|Delay _returnvalue)
      (goto _label Reset))))

(event Custom|OutFire
  (Utilities|Time|ClearandInvalidateTimerbyHandle (stale Custom|ReFire _returnvalue_2)))

(fn ConstructionScript)