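; BP_Rifle is the hero's automatic rifle, spawning bullets and spending ammo held in slot 3 of the MainGameInstance arrays.
; FireRifle checks ammo, fires immediately, then starts a looping timer at the stored fire rate, with a DoOnce and Delay limiting retriggers to one shot interval.
; Each shot spawns BP_Bullet_Hero at the Arrow, plays the hero montage and a sound at world origin.
; OutFire or empty ammo clears the timer.
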(event Custom|LoopRifle
  (bind _instanceref (Variables|Default|GetInstanceRef))
  (bind _ammo_all (Variables|/Game/Blueprints/ThirdPersonBP/Blueprints/MainGameInstance.MainGameInstance_C|GetAmmo_All _instanceref))
  (bind _output (Utilities|Array|Get(acopy) _ammo_all 3))
  (Game|SpawnActorfromClass "/Game/Blueprints/Weapon/BlueprintsBullet/BP_Bullet_Hero.BP_Bullet_Hero_C" (Transformation|GetWorldTransform (Variables|Default|GetArrow)) "Undefined" 0 0)
  (Animation|PlayAnimMontage (Variables|Default|GetHeroRef) "/Game/Characters/Hero/Animations/Fire_AnimMontage.Fire_AnimMontage" 1.0 "None")
  (bind _result (Math|Integer|DecrementInt _output)
    (:%20%20
      (Utilities|Array|SetArrayElem _ammo_all 3 _result)
      (Audio|PlaySoundatLocation "/Game/SciFiWeapLight/Sound/Rifle/Rifle_Fire_Cue.Rifle_Fire_Cue" "0, 0, 0" "0, 0, 0" 0.1 1.0 0.0 0 0 0)
      (if (<= _output 0)
        (Utilities|Time|ClearandInvalidateTimerbyHandle (stale Custom|FireRifle _returnvalue))))))

(event Custom|FireRifle
  (if (> (Utilities|Array|Get(acopy) (Variables|/Game/Blueprints/ThirdPersonBP/Blueprints/MainGameInstance.MainGameInstance_C|GetAmmo_All (Variables|Default|GetInstanceRef)) 3) 0)
    (Variables|Default|SetSpeed (Utilities|Array|Get(acopy) (Variables|/Game/Blueprints/ThirdPersonBP/Blueprints/MainGameInstance.MainGameInstance_C|GetAll_SpeedFireWeapon (Variables|Default|GetInstanceRef)) 3))
    (Utilities|FlowControl|DoOnce false :!label _label
      (:Completed
        (CallFunction|LoopRifle)
        (bind _returnvalue (Utilities|Time|SetTimerbyEvent (delegate Custom|LoopRifle) (/ 1.0 (Variables|Default|GetSpeed)) true))
        (Utilities|FlowControl|Delay (/ 1.0 (Variables|Default|GetSpeed)))
        (goto _label Reset)))))

(event Custom|OutFire
  (Utilities|Time|ClearandInvalidateTimerbyHandle (stale Custom|FireRifle _returnvalue)))

(event EventBeginPlay
  (bind _asmain_game_instance (Utilities|Casting|CastToMainGameInstance (Game|GetGameInstance)))
  (Variables|Default|SetInstanceRef _asmain_game_instance)
  (bind _asbp_hero_character (Utilities|Casting|CastToBp_HeroCharacter (Game|GetPlayerCharacter 0)))
  (Variables|Default|SetHeroRef _asbp_hero_character))

(fn ConstructionScript)