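; Shotgun weapon Blueprint that fires spread volleys of hero bullets using fire rate and ammo from the shotgun slot in MainGameInstance.
; FireShotgun fires at once and starts a looping timer, with a DoOnce and Delay limiting retriggers to the fire rate; nothing here clears the timer.
; Each shot spawns six bullets with random pitch/yaw spread, attached muzzle VFX and sound, then decrements ammo without checking it.
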(event Custom|LoopShotgun
  (bind _instanceref (Variables|Default|GetInstanceRef))
  (bind _ammo_all (Variables|/Game/Blueprints/ThirdPersonBP/Blueprints/MainGameInstance.MainGameInstance_C|GetAmmo_All _instanceref))
  (CallFunction|BulletFire)
  (bind _result (Math|Integer|DecrementInt (Utilities|Array|Get(acopy) _ammo_all 4))
    (:%20%20
      (Utilities|Array|SetArrayElem _ammo_all 4 _result))))

(event Custom|FireShotgun
  (Variables|Default|SetSpeed (Utilities|Array|Get(acopy) (Variables|/Game/Blueprints/ThirdPersonBP/Blueprints/MainGameInstance.MainGameInstance_C|GetAll_SpeedFireWeapon (Variables|Default|GetInstanceRef)) 4))
  (Utilities|FlowControl|DoOnce false :!label _label
    (:Completed
      (CallFunction|LoopShotgun)
      (Utilities|Time|SetTimerbyEvent (delegate Custom|LoopShotgun) (/ 1.0 (Variables|Default|GetSpeed)) true)
      (Utilities|FlowControl|Delay (/ 1.0 (Variables|Default|GetSpeed)))
      (goto _label Reset))))

(event Custom|BulletFire
  (bind _arrow (Variables|Default|GetArrow))
  (bind _arrow_2 (Variables|Default|GetArrow))
  (bind _min (Variables|Default|GetMin))
  (bind _max (Variables|Default|GetMax))
  (bind _returnvalue (Transformation|GetWorldLocation _arrow))
  (bind _returnvalue_2 (Transformation|GetWorldRotation _arrow))
  (Utilities|FlowControl|Sequence
    (:then_0
      (Game|SpawnActorfromClass "/Game/Blueprints/Weapon/BlueprintsBullet/BP_Bullet_Hero.BP_Bullet_Hero_C" (Math|Transform|MakeTransform _returnvalue (Math|Rotator|MakeRotator (.roll _returnvalue_2) (+ (.pitch _returnvalue_2) (Math|Random|RandomFloatinRange _min _max)) (+ (.yaw _returnvalue_2) (Math|Random|RandomFloatinRange _min _max))) "1,1,1") "Undefined" 0 0)
      (Game|SpawnActorfromClass "/Game/Blueprints/Weapon/BlueprintsBullet/BP_Bullet_Hero.BP_Bullet_Hero_C" (Math|Transform|MakeTransform _returnvalue (Math|Rotator|MakeRotator (.roll _returnvalue_2) (+ (.pitch _returnvalue_2) (Math|Random|RandomFloatinRange _min _max)) (+ (.yaw _returnvalue_2) (Math|Random|RandomFloatinRange _min _max))) "1,1,1") "Undefined" 0 0)
      (Game|SpawnActorfromClass "/Game/Blueprints/Weapon/BlueprintsBullet/BP_Bullet_Hero.BP_Bullet_Hero_C" (Math|Transform|MakeTransform _returnvalue (Math|Rotator|MakeRotator (.roll _returnvalue_2) (+ (.pitch _returnvalue_2) (Math|Random|RandomFloatinRange _min _max)) (+ (.yaw _returnvalue_2) (Math|Random|RandomFloatinRange _min _max))) "1,1,1") "Undefined" 0 0))
    (:then_1
      (Game|SpawnActorfromClass "/Game/Blueprints/Weapon/BlueprintsBullet/BP_Bullet_Hero.BP_Bullet_Hero_C" (Math|Transform|MakeTransform _returnvalue (Math|Rotator|MakeRotator (.roll _returnvalue_2) (+ (.pitch _returnvalue_2) (Math|Random|RandomFloatinRange _min _max)) (+ (.yaw _returnvalue_2) (Math|Random|RandomFloatinRange _min _max))) "1,1,1") "Undefined" 0 0)
      (Game|SpawnActorfromClass "/Game/Blueprints/Weapon/BlueprintsBullet/BP_Bullet_Hero.BP_Bullet_Hero_C" (Math|Transform|MakeTransform _returnvalue (Math|Rotator|MakeRotator (.roll _returnvalue_2) (+ (.pitch _returnvalue_2) (Math|Random|RandomFloatinRange _min _max)) (+ (.yaw _returnvalue_2) (Math|Random|RandomFloatinRange _min _max))) "1,1,1") "Undefined" 0 0)
      (Game|SpawnActorfromClass "/Game/Blueprints/Weapon/BlueprintsBullet/BP_Bullet_Hero.BP_Bullet_Hero_C" (Math|Transform|MakeTransform _returnvalue (Math|Rotator|MakeRotator (.roll _returnvalue_2) (+ (.pitch _returnvalue_2) (Math|Random|RandomFloatinRange _min _max)) (+ (.yaw _returnvalue_2) (Math|Random|RandomFloatinRange _min _max))) "1,1,1") "Undefined" 0 0)
      (bind _returnvalue_3 (Game|SpawnActorfromClass "/Game/VFX/BlueprintsVFX/BP_ShootVFX_Hero.BP_ShootVFX_Hero_C" (Transformation|GetWorldTransform _arrow_2) "Undefined" 0 0))
      (Transformation|AttachComponentToComponent _returnvalue_3 _arrow_2 "None" "SnapToTarget" "SnapToTarget" "SnapToTarget" true)
      (Audio|PlaySoundatLocation "/Game/SFX/Weapon/Shotgun/ShotGunTest.ShotGunTest" "0, 0, 0" "0, 0, 0" 0.1 1.0 0.0 0 0 0))))

(event EventBeginPlay
  (bind _asmain_game_instance (Utilities|Casting|CastToMainGameInstance (Game|GetGameInstance)))
  (Variables|Default|SetInstanceRef _asmain_game_instance))

(fn ConstructionScript)