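; Elevator that acts as a level exit, with a sliding door and an interior check that loads LevelTestMaks.
; When HeroCharacter enters Box, a timeline raises the door mesh (StaticMesh4) from its BeginPlay position.
; A Delay on the timeline's Update pin, rather than Finished, later reverses the door and, after another pause, opens the level if the player overlaps Box1.
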(event OnComponentBeginOverlap(Box)
  (params (OverlappedComponent :type Primitive%20Component%20Object%20Reference) (OtherActor :type Actor%20Object%20Reference) (OtherComp :type Primitive%20Component%20Object%20Reference) (OtherBodyIndex :type Integer) (bFromSweep :type Boolean) (SweepResult :type Hit%20Result%20Structure%20%28by%20ref%29))
  (bind _locationdoor (Variables|Default|GetLocationDoor))
  (Utilities|Casting|CastToHeroCharacter OtherActor)
  (bind _1 (Timeline|Timeline_0 Play)
    (:Update
      (Transformation|SetRelativeLocation (Variables|Default|GetStaticMesh4) (Math|Vector|Lerp(Vector) _locationdoor (+ _locationdoor "0, 0,190.000000") _1) false false)
      (Utilities|FlowControl|Delay 4.0)
      (Utilities|FlowControl|Sequence
        (:then_0
          (Utilities|FlowControl|Delay 2.0)
          (if (Collision|IsOverlappingActor (Variables|Default|GetBox1) (Game|GetPlayerCharacter 0) :!class /Script/Engine.PrimitiveComponent)
            (Game|OpenLevel(byName) "LevelTestMaks")))
        (:then_1
          (Timeline|Timeline_0 Reverse))))))

(event Custom|Start)

(event EventBeginPlay
  (Variables|Default|SetLocationDoor (Variables|/Script/Engine.SceneComponent|GetRelativeLocation (Variables|Default|GetStaticMesh4))))

(fn ConstructionScript)