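; Turret actor that tracks the player character and shoots at it while the player is inside its detection sphere.
; Sphere overlap events toggle the target lock and start or clear a rapid looping timer that spawns Bullet actors from the Arrow's transform.
; While locked, Tick turns Cube1 toward the player on yaw only, using a look-at rotation from the turret's location.
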(event OnComponentBeginOverlap(Sphere)
  (params (OverlappedComponent :type Primitive%20Component%20Object%20Reference) (OtherActor :type Actor%20Object%20Reference) (OtherComp :type Primitive%20Component%20Object%20Reference) (OtherBodyIndex :type Integer) (bFromSweep :type Boolean) (SweepResult :type Hit%20Result%20Structure%20%28by%20ref%29))
  (if (== OtherActor (Game|GetPlayerCharacter 0))
    (Variables|Default|SetTargetLocked true)
    (CallFunction|ReFire)))

(event OnComponentEndOverlap(Sphere)
  (params (OverlappedComponent :type Primitive%20Component%20Object%20Reference) (OtherActor :type Actor%20Object%20Reference) (OtherComp :type Primitive%20Component%20Object%20Reference) (OtherBodyIndex :type Integer))
  (if (== OtherActor (Game|GetPlayerCharacter 0))
    (Variables|Default|SetTargetLocked false)
    (CallFunction|OutFire)))

(event Custom|UpdateRotation
  (Transformation|SetWorldRotation (Variables|Default|GetCube1) (Math|Rotator|MakeRotator 0.0 0.0 (.yaw (Math|Rotator|FindLookatRotation (Transformation|GetActorLocation (Components|GetOwner (Variables|Default|GetCube1))) (Transformation|GetActorLocation (Game|GetPlayerCharacter 0))))) false false))

(event Custom|Fire
  (bind _arrow (Variables|Default|GetArrow))
  (bind _returnvalue (Transformation|GetWorldTransform _arrow))
  (Game|SpawnActorfromClass "/Game/Blueprints/Weapon/Bullet.Bullet_C" (Math|Transform|MakeTransform (.location _returnvalue) (.rotation _returnvalue) "1,1,1") "Undefined" 0 0))

(event Custom|ReFire
  (bind _returnvalue (Utilities|Time|SetTimerbyEvent (delegate Custom|Fire) (/ 1.0 1e+02) true)))

(event Custom|OutFire
  (Utilities|Time|ClearandInvalidateTimerbyHandle (stale Custom|ReFire _returnvalue)))

(event EventTick
  (params (DeltaSeconds :type Float%20%28single-precision%29))
  (if (Variables|Default|GetTargetLocked)
    (CallFunction|UpdateRotation)))

(fn ConstructionScript)